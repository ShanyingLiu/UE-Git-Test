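; BP_Hopper is a hopping character with a sphere body, launched along world Y and upward by holding and releasing the Hop input.
; Tick builds JumpDist while held, flattening the sphere as wind-up, and pins the spring arm to a fixed height.
; Release scales launch velocity by the charge, provided the character is not falling.
; Timelines drive squash-and-stretch scale lerps from the stored base scale on jump and landing.
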(event `self.ReceiveBeginPlay`
  (bind _returnvalue (`GameplayStatics.GetPlayerController` 0))
  (`MovieSceneSequenceExtensions.AddPossessable` null _returnvalue)
  (`self.EnableInput` _returnvalue)
  (set `self.BaseScale` (`SceneComponent.RelativeScale3D` (`self.Sphere`))))

(event `JumpSqueeze`
  (bind (_direction _alpha) (`Timeline|JumpSqueezeAnim` :!via `PlayFromStart`)
    (:`Update`
      (`SceneComponent.SetRelativeScale3D` (`self.Sphere`) (`KismetMathLibrary.VLerp` (`self.BaseScale`) (* (`self.BaseScale`) (`self.JumpSqueezeFactor`)) _alpha)))))

(event `self.ReceiveTick`
  (params (DeltaSeconds :type "Float (single-precision)"))
  (`SceneComponent.K2_SetWorldLocation` (`self.SpringArm`) (`KismetMathLibrary.MakeVector` (.x (`SceneComponent.K2_GetComponentLocation` (`self.SpringArm`))) (.y (`SceneComponent.K2_GetComponentLocation` (`self.SpringArm`))) 50.0) false false)
  ;[1 0.7632 0.2448 0.433 14] Jump Wind-up
  (if (`self.IsHolding`)
    (bind _output_get (set `self.JumpDist` (`KismetMathLibrary.FClamp` (+ (`self.JumpDist`) 0.4) 0.0 12.5)))
    (`KismetSystemLibrary.LogString` (`KismetStringLibrary.Conv_DoubleToString` _output_get))
    (`SceneComponent.SetRelativeScale3D` (`self.Sphere`) (`KismetMathLibrary.MakeVector` (.x (`self.BaseScale`)) (.y (`self.BaseScale`)) (* (.z (`self.BaseScale`)) (/ (- 100.0 (`self.JumpDist`)) 100.0))))))

(event `InputAction|Hop`
  (params (Key :type "Key Structure"))
  (bind _returnvalue (`NavMovementComponent.IsFalling` (`self.CharacterMovement`)))
  (:`Pressed`
    (set `self.IsHolding` true)
    (set `self.JumpDist` 0.0))
  (:`Released`
    (set `self.IsHolding` false)
    (`KismetSystemLibrary.LogString` (`KismetStringLibrary.Conv_BoolToString` _returnvalue))
    (if (not _returnvalue)
      (`self.LaunchCharacter` (`KismetMathLibrary.MakeVector` 0.0 (* 20.0 (`self.JumpDist`)) (+ (* 15.0 (`self.JumpDist`)) 250.0)))
      (`self.JumpSqueeze`))))

(event `self.OnLanded`
  (params (Hit :type "HitResult Structure (by ref)"))
  ;[0.5156 0.1805 0.2165 0.37 15] Landing animation
  (bind (_direction _alpha) (`Timeline|Timeline_0` :!via `PlayFromStart`)
    (:`Update`
      (`SceneComponent.SetRelativeScale3D` (`self.Sphere`) (`KismetMathLibrary.VLerp` (`self.BaseScale`) (* (`self.BaseScale`) (`self.LandSqueezeFactor`)) _alpha)))))

(fn `UserConstructionScript`)