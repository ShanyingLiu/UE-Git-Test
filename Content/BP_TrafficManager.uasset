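; BP_TrafficManager is an actor that spawns road managers, and has an event for spawning randomized traffic cars.
; BeginPlay re-enters a delayed loop, repeatedly spawning a BP_RoadManager at the origin with an incrementing RoadIdx.
; SpawnCar, not called here, places a BP_Car on either side in a random lane with random speed, nudging it if it matches LastPlacedX.
; A timer-based SpawnRoad alternative is left disconnected.
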(event `self.ReceiveBeginPlay`
  (set `self.RoadIdx` 0)
  (for _ (range 11) :!label _label
    (`KismetSystemLibrary.Delay` (`self.Interval`))
    (`self.SpawnRoad`)
    (goto _label)))

(event `SpawnCar`
  (if (`KismetMathLibrary.RandomBool`)
    (set `self.StartposX` -500.0)
    (set `self.RotationZ` 0.0)
    (else
      (set `self.StartposX` 500.0)
      (set `self.RotationZ` 180.0)))
  (bind _output_get (set `self.CurrentPlacedX` (`KismetMathLibrary.RandomIntegerInRange` 0 20)))
  (if (== (`self.LastPlacedX`) (`self.CurrentPlacedX`))
    (`/Engine/EditorBlueprintResources/StandardMacros.IncrementInt` _output_get
      (:`  `
        _)))
  (bind _returnvalue (`|SpawnActorFromClass` "/Game/BP_Car.BP_Car_C" (`KismetMathLibrary.MakeTransform` (`KismetMathLibrary.MakeVector` (`self.StartposX`) (`KismetMathLibrary.Conv_IntToDouble` (* (`self.CurrentPlacedX`) 150))) (`KismetMathLibrary.RotatorFromAxisAndAngle` (`KismetMathLibrary.MakeVector` 0.0 0.0 (`self.RotationZ`)) 180.0)) "Undefined" "MultiplyWithRoot" null null))
  (`/Engine/EditorBlueprintResources/StandardMacros.IncrementInt` (`self.SpawnNum`)
    (:`  `
      (set `/Game/BP_Car.Speed` (`KismetMathLibrary.RandomFloatInRange` 80.0 200.0) _returnvalue))))

(event `SpawnRoad`
  (bind _roadidx (`self.RoadIdx`))
  (bind _returnvalue (`|SpawnActorFromClass` "/Game/BP_RoadManager.BP_RoadManager_C" (`KismetMathLibrary.Conv_VectorToTransform` (0.0 0.0 0.0)) "Undefined" "MultiplyWithRoot" null null))
  (`KismetSystemLibrary.LogString` "Hello")
  (set `/Game/BP_RoadManager.RoadIdx` _roadidx _returnvalue)
  (`KismetSystemLibrary.LogString` (`KismetStringLibrary.Concat_StrStr` (`KismetStringLibrary.Conv_IntToString` _roadidx) "Hey what the hell"))
  (`/Engine/EditorBlueprintResources/StandardMacros.IncrementInt` (`self.RoadIdx`)))

(fn `UserConstructionScript`)