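; BP_Block is a platform in an endless hopping game that chains the next block and awards points to the player's BP_Hopper.
; On BeginPlay it randomly varies the scale of its Cylinder.
; Its first Hit spawns another BP_Block at a random distance along +Y and adds a point, with a flag preventing repeats.
; Tick destroys the block once the player moves too far away.
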(event `self.ReceiveBeginPlay`
  (bind _returnvalue (`KismetMathLibrary.RandomFloatInRange` 0.5 1.5))
  (set `self.NextGenerated` false)
  (`SceneComponent.SetRelativeScale3D` (`self.Cylinder`) (`KismetMathLibrary.MakeVector` (* (.x (`SceneComponent.RelativeScale3D` (`self.Cylinder`))) _returnvalue) (* (.y (`SceneComponent.RelativeScale3D` (`self.Cylinder`))) _returnvalue) (* (.z (`SceneComponent.RelativeScale3D` (`self.Cylinder`))) (`KismetMathLibrary.RandomFloatInRange` 0.7 1.2)))))

(event `self.ReceiveTick`
  (params (DeltaSeconds :type "Float (single-precision)"))
  (if (> (`self.GetDistanceTo` (`GameplayStatics.GetPlayerCharacter` 0)) 600.0)
    (`self.K2_DestroyActor`)))

(event `self.ReceiveHit`
  (params (MyComp :type "PrimitiveComponent Object Reference") (Other :type "Actor Object Reference") (OtherComp :type "PrimitiveComponent Object Reference") (bSelfMoved :type Boolean) (HitLocation :type "Vector Structure") (HitNormal :type "Vector Structure") (NormalImpulse :type "Vector Structure") (Hit :type "HitResult Structure (by ref)"))
  (`KismetSystemLibrary.LogString` "overlap!!!!")
  (`self.NextBlock`))

(event `NextBlock`
  (if (not (`self.NextGenerated`))
    (`|SpawnActorFromClass` "BP_Block_C" (`KismetMathLibrary.MakeTransform` (`KismetMathLibrary.MakeVector` (.x (.location (`self.GetTransform`))) (+ (.y (.location (`self.GetTransform`))) (`KismetMathLibrary.RandomFloatInRange` 90.0 350.0)) (.z (.location (`self.GetTransform`))))) "Undefined" "MultiplyWithRoot" null null)
    (set `self.NextGenerated` true)
    (bind _asbp_hopper (cast `/Game/BP_Hopper` (`GameplayStatics.GetPlayerCharacter` 0)))
    (`/Engine/EditorBlueprintResources/StandardMacros.IncrementInt` (`/Game/BP_Hopper.Points` _asbp_hopper))))

(fn `UserConstructionScript`)